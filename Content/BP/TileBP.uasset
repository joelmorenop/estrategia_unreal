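; TileBP is a clickable sprite tile that reports pointer interaction to the GMBBP game mode.
; It caches the game mode on BeginPlay, then forwards click, cursor-over and cursor-exit events from its PaperSprite to that mode's click, hover and deselect handlers, passing itself.
; It holds no selection logic of its own and exposes SetColor to tint the sprite.
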(event `self.ReceiveBeginPlay`
  (bind _asgmbbp (cast `/Game/BP/GMBBP` (`GameplayStatics.GetGameMode`)))
  (set `self.As GMBBP` _asgmbbp))

(event `self.PaperSprite.OnClicked`
  (params (TouchedComponent :type "PrimitiveComponent Object Reference") (ButtonPressed :type "Key Structure"))
  (`/Game/BP/GMBBP.On Click Tile BP` (`self.As GMBBP`) self))

(event `self.PaperSprite.OnBeginCursorOver`
  (params (TouchedComponent :type "PrimitiveComponent Object Reference"))
  (`/Game/BP/GMBBP.OnHoverTileBP` (`self.As GMBBP`) self))

(event `self.PaperSprite.OnEndCursorOver`
  (params (TouchedComponent :type "PrimitiveComponent Object Reference"))
  (`/Game/BP/GMBBP.OnDeselectTileBP` (`self.As GMBBP`) self))

(fn `SetColor`
  (params (inColor :type "LinearColor Structure"))
  (`PaperSpriteComponent.SetSpriteColor` (`self.PaperSprite`) inColor))

(fn `UserConstructionScript`)