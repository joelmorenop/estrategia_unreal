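; Game mode for a tower defense game, managing tile selection, turret placement, enemy respawn and restart on player death.
; On BeginPlay it enables mouse input, builds a list of basic, fast and missile turrets, and adds the towers HUD.
; Tiles recolor on hover and selection, turret buttons are generated from the list, and CreateTurret replaces the selected tile with a turret.
; CheckEnemyLeft triggers a respawn when no enemies remain.
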(event `self.ReceiveBeginPlay`
  (`self.SetPlayerControllerVars`)
  (`self.MakeTurretList`)
  (`self.AddHUD`))

(event `CheckEnemyLeft`
  ;[1 1 1] Custom event to respawn enemies if the quantity of them is 0
  (if (== (`self.EnemyAlive`) 0)
    (`self.RespawnEnemy`)))

(fn `AddHUD`
  ;[1 1 1] Add towers to HUD
  (bind _returnvalue (`|CreateWidget` "/Game/HUD/TowersHUDBP.TowersHUDBP_C"))
  (if (not (`Widget.IsInViewport` _returnvalue))
    (`UserWidget.AddToViewport` _returnvalue 0)))

(fn `Create Turret`
  (params (InTurret :type "/Game/BP/Turret/TurretData Object Reference"))
  (bind _actualtilebp (`self.ActualTileBP`))
  ;[0.4947 0.9301 1] Create turret on selected tile and destroy the tile
  (`/Engine/EditorBlueprintResources/StandardMacros.IsValid` _actualtilebp
    (:`Is Valid`
      (`|ExecutionSequence`
        (:`then_0`
          (bind _returnvalue (`|SpawnActorFromClass` "/Game/BP/Turret/TurretPawnBP.TurretPawnBP_C" (`self.GetTransform` _actualtilebp) "AlwaysSpawn" "OverrideRootScale" null null))
          (`/Game/BP/Turret/TurretPawnBP.Set Turret` _returnvalue InTurret))
        (:`then_1`
          (`self.K2_DestroyActor` _actualtilebp))))))

(fn `Fill Turret List`
  ;[1 0.6092 0.4268] For each turret construct a button
  (for _array_element (`self.Turret List`)
    (bind _returnvalue (`|GenericCreateObject` "/Game/HUD/BetterButton.BetterButton_C"))
    (`|ExecutionSequence`
      (:`then_0`
        (set `/Game/HUD/BetterButton.TurretComp` _array_element _returnvalue)
        (`VerticalBox.AddChildToVerticalBox` (`self.TurretPanel`) _returnvalue)
        (`/Game/HUD/BetterButton.BindOnClick` _returnvalue null))
      (:`then_1`
        (bind _returnvalue_2 (`|GenericCreateObject` "/Script/UMG.HorizontalBox"))
        (`PanelWidget.AddChild` _returnvalue _returnvalue_2)
        (`|ExecutionSequence`
          (:`then_0`
            ;[0.3604 0.9302 1] Set the turret image to the HUD (turret selection)
            (bind _returnvalue_3 (`|GenericCreateObject` "/Script/UMG.Image"))
            (`Image.SetBrush` _returnvalue_3 (`PaperSpriteBlueprintLibrary.MakeBrushFromSprite` (`/Game/BP/Turret/TurretData.TurretSprite` _array_element) 32 32))
            (`HorizontalBox.AddChildToHorizontalBox` _returnvalue_2 _returnvalue_3))
          (:`then_1`
            ;[0.503 1 0.4351] Space between turret image and name (turret selection)
            (bind _returnvalue_4 (`|GenericCreateObject` "/Script/UMG.Spacer"))
            (`Spacer.SetSize` _returnvalue_4 (20.0 20.0))
            (`HorizontalBox.AddChildToHorizontalBox` _returnvalue_2 _returnvalue_4))
          (:`then_2`
            ;[0.8408 1 0.5015] Add turret name text to the HUD (turret selection)
            (bind _returnvalue_5 (`|GenericCreateObject` "/Script/UMG.TextBlock"))
            (`TextBlock.SetText` _returnvalue_5 (`/Game/BP/Turret/TurretData.TurretName` _array_element))
            (`HorizontalBox.AddChildToHorizontalBox` _returnvalue_2 _returnvalue_5)))))))

(fn `MakeTurretList`
  (locals (NewLocalVar_0 :type "Array of /Game/BP/Turret/TurretData Object Reference"))
  (bind _turret_list (`self.Turret List`))
  ;[1 1 1] Fill the turret list
  (bind _returnvalue (`AddComponent|NODE_AddBasicTurret-0`))
  (`KismetArrayLibrary.Array_Add` _turret_list _returnvalue)
  (bind _returnvalue_2 (`AddComponent|NODE_AddFastTurret-0`))
  (`KismetArrayLibrary.Array_Add` _turret_list _returnvalue_2)
  (bind _returnvalue_3 (`AddComponent|NODE_AddMissilTurret-0`))
  (`KismetArrayLibrary.Array_Add` _turret_list _returnvalue_3))

(fn `On Click Tile BP`
  (params (TileTarget :type "/Game/BP/TileBP Object Reference"))
  ;[0.6678 1 0.7297] Deselect old and select new
  (bind _output_get (set `self.LastTileBP` (`self.ActualTileBP`)))
  (`/Engine/EditorBlueprintResources/StandardMacros.IsValid` _output_get
    (:`Is Valid`
      (`self.OnDeselectTileBP` _output_get))
    (:`Is Not Valid`
      _))
  (bind _output_get_2 (set `self.ActualTileBP` TileTarget))
  (`/Game/BP/TileBP.SetColor` _output_get_2 (`self.SelectedColor`)))

(fn `OnDeselectTileBP`
  (params (TileTarget :type "/Game/BP/TileBP Object Reference"))
  ;[1 1 1] When deselect tile change the color
  (if (not (and (== TileTarget (`self.ActualTileBP`)) (`KismetMathLibrary.LinearColor_IsNearEqual` (`PaperSpriteComponent.SpriteColor` (`/Game/BP/TileBP.PaperSprite` TileTarget)) (`self.SelectedColor`))))
    (`/Game/BP/TileBP.SetColor` TileTarget (`self.BaseColor`))))

(fn `OnHoverTileBP`
  (params (TileTarget :type "/Game/BP/TileBP Object Reference"))
  ;[1 1 1] When hover the tile change the color
  (if (not (== TileTarget (`self.ActualTileBP`)))
    (`/Game/BP/TileBP.SetColor` TileTarget (`self.HoverColor`))))

(fn `RestartoGame`
  (params (IsPlayerAlive :type Boolean))
  ;[1 0.5249 0.4651] If player is dead, restart the game
  (if (not IsPlayerAlive)
    (`self.RestartGame`)))

(fn `SetPlayerControllerVars`
  (bind _returnvalue (`GameplayStatics.GetPlayerController` 0))
  ;[1 0.6866 0.7672] Set player controller vars so the player can use the mouse
  (set `PlayerController.bShowMouseCursor` true _returnvalue)
  (set `PlayerController.bEnableClickEvents` true _returnvalue)
  (set `PlayerController.bEnableMouseOverEvents` true _returnvalue)
  (set `PlayerController.bEnableTouchOverEvents` true _returnvalue))

(fn `UserConstructionScript`)