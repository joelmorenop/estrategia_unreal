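; TurretPawnBP is a turret pawn that takes its data and Paper2D sprite appearance from a turret component assigned at runtime.
; SetTurret adds a new component of the input turret's class and stores it as TurretData, so only the class of the input is used.
; It then marks that data active, links it back to the pawn and applies its sprite.
; The event graph and construction script are empty.
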(fn `Set Turret`
  (params (`In Turret` :type "/Game/BP/Turret/TurretData Object Reference"))
  ;[1 1 1] Set the turret data
  (bind _returnvalue (`|AddComponentByClass` self (`GameplayStatics.GetObjectClass` `In Turret`)))
  (bind _output_get (set `self.TurretData` _returnvalue))
  (`|ExecutionSequence`
    (:`then_0`
      (set `/Game/BP/Turret/TurretData.TurretActive` true _output_get))
    (:`then_1`
      (set `/Game/BP/Turret/TurretData.TurretActor` self _output_get))
    (:`then_2`
      (`PaperSpriteComponent.SetSprite` (`self.PaperSprite`) (`/Game/BP/Turret/TurretData.TurretSprite` _output_get)))))

(fn `UserConstructionScript`)